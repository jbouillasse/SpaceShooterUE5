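; BP_Spaceship is the spaceship Blueprint that connects score and life changes to the on-screen HUD.
; On BeginPlay it switches the first player controller to game-only input, hides the mouse cursor, then creates WBP_HUD and adds it to the viewport.
; Its OnScoreChanged and OnLifeChanged events pass score, multiplier and lives to the widget's French-named update functions, converting them to 64-bit integers.
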(event `self.ReceiveBeginPlay`
  (bind _returnvalue (`GameplayStatics.GetPlayerController` 0))
  (`WidgetBlueprintLibrary.SetInputMode_GameOnly` _returnvalue)
  (set `PlayerController.bShowMouseCursor` false _returnvalue)
  (bind _returnvalue_2 (`|CreateWidget` "/Game/WBP_HUD.WBP_HUD_C"))
  (bind _output_get (set `self.HUD_Ref` _returnvalue_2))
  (`UserWidget.AddToViewport` _output_get 0))

(event `self.OnScoreChanged`
  (params (NewScore :type Integer) (CurrentMultiplier :type Integer))
  (`/Game/WBP_HUD.ActualiserScore` (`self.HUD_Ref`) (`KismetMathLibrary.Conv_IntToInt64` NewScore) (`KismetMathLibrary.Conv_IntToInt64` CurrentMultiplier)))

(event `self.OnLifeChanged`
  (params (CurrentLives :type Integer))
  (`/Game/WBP_HUD.ActualiserVies` (`self.HUD_Ref`) (`KismetMathLibrary.Conv_IntToInt64` CurrentLives)))

(fn `UserConstructionScript`)